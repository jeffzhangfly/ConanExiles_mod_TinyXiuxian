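; Mod controller for the TinyXiuxian mod (apparently Conan Exiles) that injects its items and loot into the game's data tables.
; ModDataTableOperations merges the mod's items into ItemTable, then removes one row by ID.
; It adds the mod's resource tables to tiered resource and repair kit tables, and Lingshi loot to many boss tables plus P_LC_Legendary.
; The event graph and construction script are empty.
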(fn `ModDataTableOperations`
  (`self.MergeDataTables` "/Game/Items/ItemTable.ItemTable" "/Game/Mods/TinyXiuxian/DataTables/dt_TinyXiuxian_Items.dt_TinyXiuxian_Items")
  (`self.RemoveDataTableRows` "/Game/Items/ItemTable.ItemTable" (`|MakeArray` "53101" :!type "Name"))
  (`self.MergeDataTables` "/Game/Systems/Loot/TableSetup/W_T1Resources.W_T1Resources" "/Game/Mods/TinyXiuxian/DataTables/W_TinyXiuxian_1Resource.W_TinyXiuxian_1Resource")
  (`self.MergeDataTables` "/Game/Systems/Loot/TableSetup/W_T2Resources.W_T2Resources" "/Game/Mods/TinyXiuxian/DataTables/W_TinyXiuxian_1Resource.W_TinyXiuxian_1Resource")
  (`self.MergeDataTables` "/Game/Systems/Loot/TableSetup/W_T3Resources.W_T3Resources" "/Game/Mods/TinyXiuxian/DataTables/W_TinyXiuxian_1Resource.W_TinyXiuxian_1Resource")
  (`self.MergeDataTables` "/Game/Systems/Loot/TableSetup/P_M_ArenaMaster.P_M_ArenaMaster" "/Game/Mods/TinyXiuxian/DataTables/P_TinyXiuxian_2Lingshi_loot.P_TinyXiuxian_2Lingshi_loot")
  (`self.MergeDataTables` "/Game/Systems/Loot/TableSetup/P_M_Warmaker_WarmasterBoss.P_M_Warmaker_WarmasterBoss" "/Game/Mods/TinyXiuxian/DataTables/P_TinyXiuxian_2Lingshi_loot.P_TinyXiuxian_2Lingshi_loot")
  (`self.MergeDataTables` "/Game/Systems/Loot/TableSetup/P_LC_Legendary.P_LC_Legendary" "/Game/Mods/TinyXiuxian/DataTables/P_TinyXiuxian_2Lingshi_loot.P_TinyXiuxian_2Lingshi_loot")
  (`self.MergeDataTables` "/Game/Systems/Loot/TableSetup/W_LegendaryRepairKit.W_LegendaryRepairKit" "/Game/Mods/TinyXiuxian/DataTables/W_TinyXiuxian_2Resource.W_TinyXiuxian_2Resource")
  (`self.MergeDataTables` "/Game/Systems/Loot/TableSetup/W_VaultRepairKits.W_VaultRepairKits" "/Game/Mods/TinyXiuxian/DataTables/W_TinyXiuxian_2Resource.W_TinyXiuxian_2Resource")
  (`self.MergeDataTables` "/Game/Systems/Loot/TableSetup/P_M_Invader_Fighter_Boss_Khayne.P_M_Invader_Fighter_Boss_Khayne" "/Game/Mods/TinyXiuxian/DataTables/P_TinyXiuxian_2Lingshi_loot.P_TinyXiuxian_2Lingshi_loot")
  (`self.MergeDataTables` "/Game/Systems/Loot/TableSetup/P_M_Invader_Fighter_Boss_Ator.P_M_Invader_Fighter_Boss_Ator" "/Game/Mods/TinyXiuxian/DataTables/P_TinyXiuxian_2Lingshi_loot.P_TinyXiuxian_2Lingshi_loot")
  (`self.MergeDataTables` "/Game/Systems/Loot/TableSetup/P_M_DaughterOfYmir_Boss.P_M_DaughterOfYmir_Boss" "/Game/Mods/TinyXiuxian/DataTables/P_TinyXiuxian_2Lingshi_loot.P_TinyXiuxian_2Lingshi_loot")
  (`self.MergeDataTables` "/Game/Systems/Loot/TableSetup/P_M_Black_Corsairs_Fighter_Boss_Zabweth.P_M_Black_Corsairs_Fighter_Boss_Zabweth" "/Game/Mods/TinyXiuxian/DataTables/P_TinyXiuxian_2Lingshi_loot.P_TinyXiuxian_2Lingshi_loot")
  (`self.MergeDataTables` "/Game/Systems/Loot/TableSetup/P_M_Black_Corsairs_Fighter_Boss_Nruka.P_M_Black_Corsairs_Fighter_Boss_Nruka" "/Game/Mods/TinyXiuxian/DataTables/P_TinyXiuxian_2Lingshi_loot.P_TinyXiuxian_2Lingshi_loot")
  (`self.MergeDataTables` "/Game/Systems/Loot/TableSetup/P_M_Invader_Fighter_Boss_Kraxus.P_M_Invader_Fighter_Boss_Kraxus" "/Game/Mods/TinyXiuxian/DataTables/P_TinyXiuxian_2Lingshi_loot.P_TinyXiuxian_2Lingshi_loot")
  (`self.MergeDataTables` "/Game/Systems/Loot/TableSetup/P_M_Invader_Fighter_Boss_Minstrel.P_M_Invader_Fighter_Boss_Minstrel" "/Game/Mods/TinyXiuxian/DataTables/P_TinyXiuxian_2Lingshi_loot.P_TinyXiuxian_2Lingshi_loot")
  (`self.MergeDataTables` "/Game/Systems/Loot/TableSetup/P_M_JhilBoss.P_M_JhilBoss" "/Game/Mods/TinyXiuxian/DataTables/P_TinyXiuxian_2Lingshi_loot.P_TinyXiuxian_2Lingshi_loot")
  (`self.MergeDataTables` "/Game/Systems/Loot/TableSetup/P_M_Relic_Boss.P_M_Relic_Boss" "/Game/Mods/TinyXiuxian/DataTables/P_TinyXiuxian_2Lingshi_loot.P_TinyXiuxian_2Lingshi_loot")
  (`self.MergeDataTables` "/Game/Systems/Loot/TableSetup/P_M_Accursed_Fighter_Boss_Calandra.P_M_Accursed_Fighter_Boss_Calandra" "/Game/Mods/TinyXiuxian/DataTables/P_TinyXiuxian_2Lingshi_loot.P_TinyXiuxian_2Lingshi_loot")
  (`self.MergeDataTables` "/Game/Systems/Loot/TableSetup/P_M_Accursed_Fighter_Boss_TheNameLessShadow.P_M_Accursed_Fighter_Boss_TheNameLessShadow" "/Game/Mods/TinyXiuxian/DataTables/P_TinyXiuxian_2Lingshi_loot.P_TinyXiuxian_2Lingshi_loot")
  (`self.MergeDataTables` "/Game/Systems/Loot/TableSetup/P_M_Accursed_Fighter_Boss_Ridrik.P_M_Accursed_Fighter_Boss_Ridrik" "/Game/Mods/TinyXiuxian/DataTables/P_TinyXiuxian_2Lingshi_loot.P_TinyXiuxian_2Lingshi_loot")
  (`self.MergeDataTables` "/Game/Systems/Loot/TableSetup/P_M_Accursed_Fighter_Boss_RebelJin.P_M_Accursed_Fighter_Boss_RebelJin" "/Game/Mods/TinyXiuxian/DataTables/P_TinyXiuxian_2Lingshi_loot.P_TinyXiuxian_2Lingshi_loot")
  (`self.MergeDataTables` "/Game/Systems/Loot/TableSetup/P_M_Accursed_Fighter_Boss_Petr.P_M_Accursed_Fighter_Boss_Petr" "/Game/Mods/TinyXiuxian/DataTables/P_TinyXiuxian_2Lingshi_loot.P_TinyXiuxian_2Lingshi_loot")
  (`self.MergeDataTables` "/Game/Systems/Loot/TableSetup/P_M_Accursed_Fighter_Boss_NL3.P_M_Accursed_Fighter_Boss_NL3" "/Game/Mods/TinyXiuxian/DataTables/P_TinyXiuxian_2Lingshi_loot.P_TinyXiuxian_2Lingshi_loot")
  (`self.MergeDataTables` "/Game/Systems/Loot/TableSetup/P_M_Accursed_Fighter_Boss_NL2.P_M_Accursed_Fighter_Boss_NL2" "/Game/Mods/TinyXiuxian/DataTables/P_TinyXiuxian_2Lingshi_loot.P_TinyXiuxian_2Lingshi_loot")
  (`self.MergeDataTables` "/Game/Systems/Loot/TableSetup/P_M_Accursed_Fighter_Boss_NL1.P_M_Accursed_Fighter_Boss_NL1" "/Game/Mods/TinyXiuxian/DataTables/P_TinyXiuxian_2Lingshi_loot.P_TinyXiuxian_2Lingshi_loot")
  (`self.MergeDataTables` "/Game/Systems/Loot/TableSetup/P_M_Black_Corsairs_Fighter_Boss_NL1.P_M_Black_Corsairs_Fighter_Boss_NL1" "/Game/Mods/TinyXiuxian/DataTables/P_TinyXiuxian_2Lingshi_loot.P_TinyXiuxian_2Lingshi_loot")
  (`self.MergeDataTables` "/Game/Systems/Loot/TableSetup/P_M_Invader_Fighter_Boss_NL1.P_M_Invader_Fighter_Boss_NL1" "/Game/Mods/TinyXiuxian/DataTables/P_TinyXiuxian_2Lingshi_loot.P_TinyXiuxian_2Lingshi_loot")
  (`self.MergeDataTables` "/Game/Systems/Loot/TableSetup/P_M_Black_Corsairs_Fighter_Boss_NL2.P_M_Black_Corsairs_Fighter_Boss_NL2" "/Game/Mods/TinyXiuxian/DataTables/P_TinyXiuxian_2Lingshi_loot.P_TinyXiuxian_2Lingshi_loot")
  (`self.MergeDataTables` "/Game/Systems/Loot/TableSetup/P_M_Invader_Fighter_Boss_NL2.P_M_Invader_Fighter_Boss_NL2" "/Game/Mods/TinyXiuxian/DataTables/P_TinyXiuxian_2Lingshi_loot.P_TinyXiuxian_2Lingshi_loot")
  (`self.MergeDataTables` "/Game/Systems/Loot/TableSetup/P_M_Black_Corsairs_Fighter_Boss_NL3.P_M_Black_Corsairs_Fighter_Boss_NL3" "/Game/Mods/TinyXiuxian/DataTables/P_TinyXiuxian_2Lingshi_loot.P_TinyXiuxian_2Lingshi_loot")
  (`self.MergeDataTables` "/Game/Systems/Loot/TableSetup/P_M_Invader_Fighter_Boss_NL3.P_M_Invader_Fighter_Boss_NL3" "/Game/Mods/TinyXiuxian/DataTables/P_TinyXiuxian_2Lingshi_loot.P_TinyXiuxian_2Lingshi_loot"))

(fn `UserConstructionScript`)